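; BP_Personaje is a player-controlled character, animated by ABP_Paladin, with movement, mouse look, jump and a grounded attack.
; Axis inputs move it relative to the controller's rotation and turn the view.
; Attacking checks the falling state through the anim Blueprint's movement reference, then stops and disables movement while IsAttacking is set.
; A fixed delay, rather than an animation event, ends the attack and restores walking.
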(event Input|ActionEvents|InputActionSalto
  (params (Key :type Key%20Structure :default "None"))
  (:Pressed
    (Character|Jump))
  (:Released
    (Character|StopJumping)))

(event Input|ActionEvents|InputActionAtacar
  (params (Key :type Key%20Structure :default "None"))
  (bind _charactermovement (Variables|Character|GetCharacterMovement))
  (:Pressed
    (bind _asabp_paladin (Utilities|Casting|CastToABP_Paladin (Components|SkeletalMesh|GetAnimInstance (Variables|Character|GetMesh))))
    (if (not (AI|Components|NavMovement|IsFalling (Variables|/Game/Anim/ABP_Paladin.ABP_Paladin_C|GetCharacter%20Movement _asabp_paladin)))
      (Components|Movement|StopMovementImmediately _charactermovement)
      (Pawn|Components|CharacterMovement|DisableMovement _charactermovement)
      (Variables|Default|SetIsAttacking? true)
      (Utilities|FlowControl|Delay 1.4)
      (Variables|Default|SetIsAttacking? false)
      (Pawn|Components|CharacterMovement|SetMovementMode (Variables|Character|GetCharacterMovement) "MOVE_Walking" 0))))

(event Input|AxisEvents|InputAxisIzquierda-Derecha
  (params (AxisValue :type Float%20%28single-precision%29))
  (bind _returnvalue (Pawn|GetControlRotation :!class /Script/Engine.Pawn))
  ;[0.15 0.15 0.15 0.5] KeyBoards A/D
  (Pawn|Input|AddMovementInput (Math|Vector|GetRightVector (Math|Rotator|MakeRotator (.roll _returnvalue) 0.0 (.yaw _returnvalue))) AxisValue false))

(event Input|AxisEvents|InputAxisDelante-Atras
  (params (AxisValue :type Float%20%28single-precision%29))
  ;[0.15 0.15 0.15 0.5] KeyBoards W/S
  (Pawn|Input|AddMovementInput (Math|Vector|GetForwardVector (Math|Rotator|MakeRotator 0.0 0.0 (.yaw (Pawn|GetControlRotation :!class /Script/Engine.Pawn)))) AxisValue false))

(event Input|AxisEvents|InputAxisMouseArriba-Abajo
  (params (AxisValue :type Float%20%28single-precision%29))
  ;[0.15 0.15 0.15 0.5] Mouse UP/DOWN
  (Pawn|Input|AddControllerPitchInput AxisValue))

(event Input|AxisEvents|InputAxisMouseIzquierda-Derecha
  (params (AxisValue :type Float%20%28single-precision%29))
  ;[0.15 0.15 0.15 0.5] Mouse LEFT/RIGHT
  (Pawn|Input|AddControllerYawInput AxisValue))

(fn ConstructionScript)